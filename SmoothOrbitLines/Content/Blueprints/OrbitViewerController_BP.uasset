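; OrbitViewerController_BP is a controller that sets up the HUD for an orbit viewer.
; On BeginPlay it caches every OrbitingBody actor in Bodies, then creates the HUD overlay widget.
; It hands the widget references to itself and the GameState, then adds it to the viewport as visible.
; Tick and the construction script are empty, and the cached Bodies list is not used within this file.
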(event `self.ReceiveBeginPlay`
  (bind _outactors (`GameplayStatics.GetAllActorsOfClass` "/Script/SmoothOrbitLines.OrbitingBody"))
  (set `self.Bodies` _outactors)
  (`self.Create HUD Overlay`))

(fn `Create HUD Overlay`
  (bind _returnvalue (`|CreateWidget` (`self.HudOverlayAsset`)))
  (bind _ashud_overlay (cast `/Game/Widget/HudOverlay` _returnvalue))
  (bind _output_get (set `self.HudOverlayInstance` _ashud_overlay))
  (set `/Game/Widget/HudOverlay.PlayerController` self _output_get)
  (set `/Game/Widget/HudOverlay.GameState` (`self.GameState`) _output_get)
  (`UserWidget.AddToViewport` _output_get 1)
  (`Widget.SetVisibility` (`self.HudOverlayInstance`) "Visible"))

(fn `UserConstructionScript`)