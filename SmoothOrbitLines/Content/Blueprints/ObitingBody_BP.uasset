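; Actor for an orbiting body in an orbit viewer, shown as a scaled mesh with an on-screen icon.
; BeginPlay caches orbit state and controller, creates the icon and computes orbit geometry from conic elements.
; Each tick, non-inertial bodies recompute their state at the current Et, and the controller maps state vectors into scene positions.
; The icon follows the projected location, hiding when projection fails; mesh scale derives from radii, scene scale and bounds.
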(event `self.ReceiveBeginPlay`
  (bind _asorbit_game_state_bp (cast `/Game/Blueprints/OrbitGameState_BP` (`GameplayStatics.GetGameState`)))
  (set `self.State` (`OrbitGameState.OrbitSystemState` _asorbit_game_state_bp))
  (bind _asorbit_viewer_controller_bp (cast `/Game/Blueprints/OrbitViewerController_BP` (`GameplayStatics.GetPlayerController` 0)))
  (set `self.Controller` (`OrbitViewerController.OrbitViewerController` _asorbit_viewer_controller_bp))
  (`self.Create Icon`)
  (bind _geometry (`OrbitalMechanics.ComputeGeometry` (`OrbitingBodyComponent.ConicElements` (`self.OrbitingBody`)))
    (:`Success`
      (set `OrbitingBodyComponent.OrbitGeometry` _geometry (`self.OrbitingBody`)))))

(event `self.ReceiveTick`
  (params (DeltaSeconds :type "Float (single-precision)"))
  (`self.Update Body Location`)
  (`self.Update Icon Location`))

(fn `Create Icon`
  (`self.Set Mesh Scale`)
  (bind _returnvalue (`|CreateWidget` (`self.Icon Widget Asset`)))
  (bind _asbody_icon (cast `/Game/Widget/BodyIcon` _returnvalue))
  (bind _output_get (set `self.User Widget Instance` _asbody_icon))
  (set `/Game/Widget/BodyIcon.BodyName` (`self.BodyName`) _output_get)
  (set `/Game/Widget/BodyIcon.IconColor` (`OrbitingBodyComponent.LineColor` (`self.OrbitingBody`)) (`self.User Widget Instance`))
  (`UserWidget.AddToViewport` (`self.User Widget Instance`) 1)
  (`Widget.SetVisibility` (`self.User Widget Instance`) "Visible")
  (`UserWidget.SetAlignmentInViewport` (`self.User Widget Instance`) (0.5 0.5)))

(fn `Set Mesh Scale`
  (bind (_min _max) (`StaticMeshComponent.GetLocalBounds` (`self.Mesh`)))
  (bind _returnvalue (`KismetMathLibrary.Conv_DoubleToFloat` (`OrbitViewerControllerComponent.SceneScale` (`self.Controller`))))
  (`self.SetActorScale3D` (* (`self.Radii`) (/ (`KismetMathLibrary.MakeVector` _returnvalue _returnvalue _returnvalue) (* (- _max _min) (0.5 0.5 0.5))))))

(fn `Update Body Location`
  (if (`OrbitingBodyComponent.IsInertial` (`self.OrbitingBody`))
    (`self.K2_SetActorLocation` (`.r` (break `SceneStateVector` (`OrbitViewerControllerComponent.GetSceneStateVector` (`self.Controller`) (`.StateVector` (break `State` (`OrbitingBodyComponent.OrbitState` (`self.OrbitingBody`))))))))
    (else
      (bind _state (`OrbitalMechanics.ComputeState` (`OrbitingBodyComponent.ConicElements` (`self.OrbitingBody`)) (`OrbitSystemStateComponent.et` (`self.State`)))
        (:`Success`
          (bind _output_get (set `OrbitingBodyComponent.OrbitState` _state (`self.OrbitingBody`)))
          (`self.K2_SetActorLocation` (`.r` (break `SceneStateVector` (`OrbitViewerControllerComponent.GetSceneStateVector` (`self.Controller`) (`.StateVector` (break `State` _output_get)))))))))))

(fn `Update Icon Location`
  (bind (_screenposition _returnvalue) (`GameplayStatics.ProjectWorldToScreen` (`GameplayStatics.GetPlayerController` 0) (`self.K2_GetActorLocation`)))
  (`UserWidget.SetPositionInViewport` (`self.User Widget Instance`) _screenposition true)
  (if _returnvalue
    (`Widget.SetVisibility` (`self.User Widget Instance`) "Visible")
    (else
      (`Widget.SetVisibility` (`self.User Widget Instance`) "Hidden"))))

(fn `Update Orbit Geometry`
  (`OrbitViewerControllerComponent.ComputeGeometry` (`self.Controller`) (`OrbitingBodyComponent.ConicElements` (`self.OrbitingBody`))))

(fn `UserConstructionScript`)