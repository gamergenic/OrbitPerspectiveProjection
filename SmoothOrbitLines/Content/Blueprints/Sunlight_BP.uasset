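; Sunlight actor Blueprint that keeps its rotation aligned to the scene position supplied by the orbit viewer controller.
; On BeginPlay it casts the first player controller to OrbitViewerController_BP and caches its OrbitViewerController object.
; Each tick it queries the scene position of a default-constructed frame position, normalizes and negates that vector, and sets the actor's X axis to the result.
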(event `self.ReceiveBeginPlay`
  (bind _asorbit_viewer_controller_bp (cast `/Game/Blueprints/OrbitViewerController_BP` (`GameplayStatics.GetPlayerController` 0)))
  (set `self.Controller` (`OrbitViewerController.OrbitViewerController` _asorbit_viewer_controller_bp)))

(event `self.ReceiveTick`
  (params (DeltaSeconds :type "Float (single-precision)"))
  (`self.K2_SetActorRotation` (`KismetMathLibrary.Conv_VectorToRotator` (`KismetMathLibrary.NegateVector` (`KismetMathLibrary.Normal` (`OrbitViewerControllerComponent.GetScenePosition` (`self.Controller`) (make `FramePosition`)))))))

(fn `UserConstructionScript`)